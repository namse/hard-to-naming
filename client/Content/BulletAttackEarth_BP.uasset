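; BulletAttackEarth_BP is an earth-themed bullet attack actor that damages characters on other teams when it overlaps them.
; On overlap it casts the other actor to Character_BP and compares that character's TeamID with its own.
; A CollidedCharacters list ensures each opposing character receives DealDamage only once.
; Debug prints show the overlapped actor's first tag and both team IDs.
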(event EventBeginPlay
  (|CallParentFunction))

(event Collision|EventActorBeginOverlap
  (params (OtherActor :type Actor%20Object%20Reference))
  (bind _teamid (Variables|Default|GetTeamID))
  (Development|PrintText (Utilities|Text|ToText(Name) (Utilities|Array|Get(acopy) (Variables|/Script/Engine.Actor|GetTags OtherActor))) true true "(R=1.000000,G=0.000000,B=0.396272,A=1.000000)" 1e+02)
  (bind _ascharacter_bp (Utilities|Casting|CastToCharacter_BP OtherActor))
  (Development|PrintString (Utilities|String|Append (Utilities|String|ToString(Integer) (Variables|/Game/Character_BP.Character_BP_C|GetTeamID _ascharacter_bp)) (Utilities|String|ToString(Integer) _teamid)))
  (Utilities|EqualBranch(Integer) (Variables|/Game/Character_BP.Character_BP_C|GetTeamID _ascharacter_bp) _teamid
    (:False
      (if (not (Utilities|Array|ContainsItem (Variables|Default|GetCollidedCharacters) _ascharacter_bp))
        (Utilities|Array|AddUnique (Variables|Default|GetCollidedCharacters) _ascharacter_bp)
        (CallFunction|DealDamage (Variables|Default|GetDamage) _ascharacter_bp)))))

(event EventTick
  (params (DeltaSeconds :type Float%20%28single-precision%29))
  (|CallParentFunction 0.0))

(fn ConstructionScript
  (|CallParentFunction))