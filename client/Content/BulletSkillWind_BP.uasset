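; BulletSkillWind_BP is a wind skill projectile that damages characters on opposing teams as it overlaps them.
; Each tick it adds Acceleration to Velocity and applies the result along its local X axis through ProjectileMovement.
; On overlap it records enemy Character_BP hits in CollidedCharacters, so each takes damage only once, and the projectile is not destroyed here.
; Debug text prints the current velocity and the overlapped actor's first tag.
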(event EventBeginPlay
  (|CallParentFunction))

(event Collision|EventActorBeginOverlap
  (params (OtherActor :type Actor%20Object%20Reference))
  (Development|PrintText (Utilities|Text|ToText(Name) (Utilities|Array|Get(acopy) (Variables|/Script/Engine.Actor|GetTags OtherActor))) true true "(R=1.000000,G=0.000000,B=0.396272,A=1.000000)" 1e+02)
  (bind _ascharacter_bp (Utilities|Casting|CastToCharacter_BP OtherActor))
  (Utilities|EqualBranch(Integer) (Variables|/Game/Character_BP.Character_BP_C|GetTeamID _ascharacter_bp) (Variables|Default|GetTeamID)
    (:False
      (if (not (Utilities|Array|ContainsItem (Variables|Default|GetCollidedCharacters) _ascharacter_bp))
        (Utilities|Array|AddUnique (Variables|Default|GetCollidedCharacters) _ascharacter_bp)
        (CallFunction|DealDamage (Variables|Default|GetDamage) _ascharacter_bp)))))

(event EventTick
  (params (DeltaSeconds :type Float%20%28single-precision%29))
  (|CallParentFunction DeltaSeconds)
  (bind _output_get (Variables|Default|SetVelocity (+ (Variables|Default|GetVelocity) (* DeltaSeconds (Variables|Default|GetAcceleration)))))
  (Game|Components|ProjectileMovement|SetVelocityinLocalSpace (Variables|Default|GetProjectileMovement) (Math|Vector|MakeVector _output_get 0.0 0.0))
  (Development|PrintText (Utilities|Text|ToText(Float) _output_get "HalfToEven") true true "(R=1.000000,G=0.000000,B=0.124062,A=1.000000)" 0.0))

(fn ConstructionScript
  (|CallParentFunction))