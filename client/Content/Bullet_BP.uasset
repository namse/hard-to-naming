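; Bullet actor that damages enemy characters on overlap and destroys itself.
; It starts hidden, then after an optional activation delay becomes visible and starts an optional lifetime timer that destroys it.
; Any overlap destroys it, but only a Character_BP with a different TeamID takes damage.
; Debug prints report activation, per-tick location and the overlapped actor's first tag.
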(event EventBeginPlay
  (Development|PrintText "begin" true true "(R=1.000000,G=0.000000,B=0.649640,A=1.000000)" 1e+02)
  (Rendering|SetActorHiddenInGame true)
  (if (> (Variables|Default|GetActivationDelay) 0.0)
    (Utilities|FlowControl|Delay (Variables|Default|GetActivationDelay))
    (CallFunction|Activate)
    (else
      (CallFunction|Activate))))

(event Collision|EventActorBeginOverlap
  (params (OtherActor :type Actor%20Object%20Reference))
  (Development|PrintText (Utilities|Text|ToText(Name) (Utilities|Array|Get(acopy) (Variables|/Script/Engine.Actor|GetTags OtherActor))) true true "(R=1.000000,G=0.000000,B=0.396272,A=1.000000)" 1e+02)
  (bind _ascharacter_bp (Utilities|Casting|CastToCharacter_BP OtherActor)
    (:then
      (Utilities|EqualBranch(Integer) (Variables|/Game/Character_BP.Character_BP_C|GetTeamID _ascharacter_bp) (Variables|Default|GetTeamID)
        (:True
          (Actor|DestroyActor))
        (:False
          (CallFunction|DealDamage (Variables|Default|GetDamage) _ascharacter_bp)
          (Actor|DestroyActor))))
    (:CastFailed
      (Actor|DestroyActor))))

(event EventTick
  (params (DeltaSeconds :type Float%20%28single-precision%29))
  (Development|PrintText (Utilities|Text|ToText(String) (Transformation|GetActorLocation)) true true "(R=0.000000,G=0.660000,B=1.000000,A=1.000000)" 0.0))

(event EventDestroyed
  (CallFunction|ClearTimer))

(fn ConstructionScript)

(fn Activate
  (Utilities|FlowControl|Sequence
    (:then_0
      (Rendering|SetActorHiddenInGame false)
      (Development|PrintText "Activate" true true "(R=1.000000,G=0.000000,B=0.649640,A=1.000000)" 1e+02))
    (:then_1
      (CallFunction|InitTimer))))

(fn ClearTimer
  (bind _timer (Variables|Default|GetTimer))
  (if (Utilities|Time|IsValidTimerHandle _timer)
    (Utilities|Time|ClearandInvalidateTimerbyHandle _timer)))

(fn OnTimer
  (Actor|DestroyActor))

(fn InitTimer
  (bind _maxduration (Variables|Default|GetMaxDuration))
  (if (> _maxduration 0.0)
    (bind _returnvalue (Utilities|Time|SetTimerbyFunctionName self "OnTimer" _maxduration))
    (Variables|Default|SetTimer _returnvalue)
    (return)
    (else
      (return))))