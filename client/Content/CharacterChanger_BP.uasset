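; CharacterChanger_BP is a trigger actor that swaps a base character for one of a configured CharacterClass.
; When an overlapping Character_BP leaves, ChangeCharacterType spawns the new class at its transform, copies TeamID, has its instigator controller possess the replacement and destroys the original.
; An exact class check limits the swap to plain Character_BP instances, excluding subclasses.
; Begin and end overlaps also print debug text.
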(event EventBeginPlay)

(event Collision|EventActorBeginOverlap
  (params (OtherActor :type Actor%20Object%20Reference))
  (Development|PrintText "Start" true true "(R=1.000000,G=0.135502,B=0.000000,A=1.000000)" 1e+02))

(event EventTick
  (params (DeltaSeconds :type Float%20%28single-precision%29)))

(event Collision|EventActorEndOverlap
  (params (OtherActor :type Actor%20Object%20Reference))
  (Development|PrintString "End" true true "(R=1.000000,G=0.000000,B=0.078177,A=1.000000)" 1e+02)
  (bind _ascharacter_bp (Utilities|Casting|CastToCharacter_BP OtherActor))
  (CallFunction|ChangeCharacterType _ascharacter_bp))

(fn ConstructionScript)

(fn ChangeCharacterType
  (params (Character :type Character%20BP%20Object%20Reference))
  (bind _output_get (LocalVariables|SetOldCharacter Character))
  (if (== "/Game/Character_BP.Character_BP_C" (Utilities|GetClass _output_get))
    (Development|PrintText (Utilities|Text|ToText(String) (Transformation|GetActorTransform (LocalVariables|GetOldCharacter))))
    (bind _returnvalue (Game|SpawnActorfromClass (Variables|Default|GetCharacterClass) (Transformation|GetActorTransform (LocalVariables|GetOldCharacter)) "AdjustIfPossibleButAlwaysSpawn" 0 0))
    (LocalVariables|SetNewCharacter _returnvalue)
    (LocalVariables|SetController (Game|GetInstigatorController (LocalVariables|GetOldCharacter)))
    (Variables|/Game/Character_BP.Character_BP_C|SetTeamID (LocalVariables|GetNewCharacter) (Variables|/Game/Character_BP.Character_BP_C|GetTeamID (LocalVariables|GetOldCharacter)))
    (Pawn|Possess (LocalVariables|GetController) (LocalVariables|GetNewCharacter))
    (Actor|DestroyActor (LocalVariables|GetOldCharacter))))