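; Earth character Blueprint that maps mouse buttons to its two earth skills.
; Left click activates SkillAttackEarthBP and right click activates SkillEarthBP, each passed a freshly generated bullet-type skill parameter.
; Both presses also print a constant false value as long-lasting on-screen text, apparently leftover debugging.
; BeginPlay, overlap and Tick are unused stubs, and construction only calls the parent.
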(event EventBeginPlay
  (|CallParentFunction))

(event Collision|EventActorBeginOverlap
  (params (OtherActor :type Actor%20Object%20Reference)))

(event EventTick
  (params (DeltaSeconds :type Float%20%28single-precision%29))
  (|CallParentFunction 0.0))

(event Input|MouseEvents|RightMouseButton
  (params (Key :type Key%20Structure :default "AnyKey"))
  (:Pressed
    (bind _skillparameter (CallFunction|GenerateSkillParameterBulletType))
    (Default|ActivateSkill (Variables|Default|GetSkillEarth_BP) _skillparameter)
    (Development|PrintText (Utilities|Text|ToText(Boolean) false) true true "(R=0.000000,G=0.660000,B=1.000000,A=1.000000)" 1e+02)))

(event Input|MouseEvents|LeftMouseButton
  (params (Key :type Key%20Structure :default "AnyKey"))
  (:Pressed
    (bind _skillparameter (CallFunction|GenerateSkillParameterBulletType))
    (Default|ActivateSkill (Variables|Default|GetSkillAttackEarth_BP) _skillparameter)
    (Development|PrintText (Utilities|Text|ToText(Boolean) false) true true "(R=0.000000,G=0.660000,B=1.000000,A=1.000000)" 1e+02)))

(fn ConstructionScript
  (|CallParentFunction))