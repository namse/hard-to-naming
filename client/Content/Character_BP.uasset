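; Replicated player character that moves on world axes, takes damage and supplies bullet spawn data for skills.
; MoveForward and MoveRight drive movement input, while Tick prints the actor's location as debug text.
; OnDamaged_Event lowers HP, or on death notifies MyPlayerController and destroys the actor.
; Helper functions flatten player 0's deprojected mouse position into a look-at rotation, offset a spawn point ahead of the capsule and pack both into a skill parameter.
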(event Custom|OnDamaged_Event
  (params (Damage :type Integer))
  ;[1 1 1] On Damaged
  (if (<= (- (Variables|Default|GetHP) Damage) 0)
    ;[1 1 1] Before Destroyed
    (Development|PrintText "Killed!")
    (bind _asmy_player_controller (Utilities|Casting|CastToMyPlayerController (Pawn|GetController))
      (:then
        (Default|OnCharacterDestroyed _asmy_player_controller))
      (:CastFailed
        _))
    (Actor|DestroyActor)
    (else
      (bind _output_get (Variables|Default|SetHP (- (Variables|Default|GetHP) Damage)))
      (Development|PrintText (Utilities|Text|ToText(String) (Utilities|String|Append "히트다 히트 " "HP : " (Utilities|String|ToString(Integer) _output_get)))))))

(event Collision|EventActorBeginOverlap
  (params (OtherActor :type Actor%20Object%20Reference)))

(event EventTick
  (params (DeltaSeconds :type Float%20%28single-precision%29))
  (Development|PrintText (Utilities|Text|ToText(String) (.location (Transformation|GetActorTransform))) true true "(R=0.000000,G=0.660000,B=1.000000,A=1.000000)" 0.0))

(event EventBeginPlay
  (Networking|SetReplicates true))

(event Input|AxisEvents|InputAxisMoveForward
  (params (AxisValue :type Float%20%28single-precision%29))
  (Pawn|Input|AddMovementInput "1.000000, 0, 0" AxisValue false))

(event Input|AxisEvents|InputAxisMoveRight
  (params (AxisValue :type Float%20%28single-precision%29))
  (Pawn|Input|AddMovementInput "0.000000,1.000000, 0" AxisValue false))

(fn ConstructionScript)

(fn GetLookatRotation
  (bind _returnvalue (Transformation|GetActorLocation))
  (bind _returnvalue_2 (Game|GetPlayerController 0))
  (bind _worldlocation (Game|Player|ConvertMouseLocationToWorldSpace _returnvalue_2))
  (return (Math|Rotator|FindLookatRotation (Math|Vector|MakeVector (.x _returnvalue) (.y _returnvalue) 0.0) (Math|Vector|MakeVector (.x _worldlocation) (.y _worldlocation) 0.0))))

(fn GetBulletStartLocation
  (params (LookAtRotation :type Rotator))
  (return (+ (* (Math|Vector|Normalize (Math|Vector|GetForwardVector LookAtRotation)) (+ (/ (Components|Capsule|GetScaledCapsuleRadius (Variables|Collision|GetCapsuleComponent)) 2.0) 1e+02)) (Transformation|GetActorLocation))))

(fn GetBulletStartTransform
  (bind _rotation (CallFunction|GetLookatRotation))
  (bind _location (CallFunction|GetBulletStartLocation _rotation))
  (return (Math|Transform|MakeTransform _location _rotation)))

(fn GenerateSkillParameterBulletType
  (Utilities|FlowControl|Sequence
    (:then_0
      (bind _transform (CallFunction|GetBulletStartTransform)))
    (:then_1
      (return (Utilities|Struct|MakeSkillParameter _transform)))))