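; A projectile bullet Blueprint that extends a parent class, using a ProjectileMovement component to fly at constant local-forward velocity once activated.
; Mesh overlap events stay off from BeginPlay until Activate enables them and sets the velocity.
; InitTimer schedules OnTimer from MaxDuration or MaxDistance divided by speed, taking the longer when both are set and skipping the timer when neither is.
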(event EventBeginPlay
  (Variables|/Script/Engine.PrimitiveComponent|SetbGenerateOverlapEvents (Variables|Character|GetMesh) false)
  (|CallParentFunction))

(event EventActivate
  (|CallParentFunction)
  (Utilities|FlowControl|Sequence
    (:then_0
      (Variables|/Script/Engine.PrimitiveComponent|SetbGenerateOverlapEvents (Variables|Character|GetMesh) true))
    (:then_1
      (Game|Components|ProjectileMovement|SetVelocityinLocalSpace (Variables|Default|GetProjectileMovement) (Math|Vector|MakeVector (Variables|Default|GetVelocity) 0.0 0.0)))))

(event EventInitTimer
  (bind (_isneedtimer _duration) (CallFunction|CalculateTimerDuration (Variables|Default|GetVelocity)))
  (if _isneedtimer
    (bind _returnvalue (Utilities|Time|SetTimerbyFunctionName self "OnTimer" _duration))
    (Variables|Default|SetTimer _returnvalue)))

(fn ConstructionScript)

(fn CalculateTimerDuration
  (params (Speed :type Float%20%28single-precision%29))
  (bind _maxdistance (Variables|Default|GetMaxDistance))
  (bind _returnvalue (/ _maxdistance Speed))
  (LocalVariables|SetHasMaxDistance (> (Variables|Default|GetMaxDistance) 0.0))
  (LocalVariables|SetHasMaxDuration (> (Variables|Default|GetMaxDuration) 0.0))
  (return (or (LocalVariables|GetHasMaxDistance) (LocalVariables|GetHasMaxDuration)) (Math|Float|SelectFloat (Variables|Default|GetMaxDuration) _returnvalue (and (or (not (LocalVariables|GetHasMaxDistance)) (> (Variables|Default|GetMaxDuration) _returnvalue)) (LocalVariables|GetHasMaxDuration)))))