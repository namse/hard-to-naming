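; SkillAttackWater_BP is a water attack skill that fires a projectile when performed.
; On OnPerformSkill it spawns BulletAttackWater_BP at the skill parameter's start transform, passing along the activator's TeamID.
; It then calls WaitPostDelay after the spawn, and also prints the start transform as text, apparently for debugging.
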(event Custom|OnPerformSkill
  (bind _skillparameter (Variables|Default|GetSkillParameter))
  (bind (_starttransform _activator) (Utilities|Struct|BreakSkillParameter _skillparameter))
  (Development|PrintText (Utilities|Text|ToText(String) _starttransform))
  (Game|SpawnActorfromClass "/Game/BulletAttackWater_BP.BulletAttackWater_BP_C" _starttransform "Undefined" 0 0.0 (Variables|/Game/Character_BP.Character_BP_C|GetTeamID _activator))
  (CallFunction|WaitPostDelay))

(event EventBeginPlay
  (|CallParentFunction))

(event EventTick
  (params (DeltaSeconds :type Float%20%28single-precision%29))
  (|CallParentFunction 0.0))