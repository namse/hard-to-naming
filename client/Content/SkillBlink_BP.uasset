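; Blink skill Blueprint that teleports the activator to the target X/Y at its current height, then waits for the post delay.
; GetAvailableBlinkLocation sphere-tests the target using the activator's capsule radius.
; If blocked, it samples rings of growing radius by angle increments until a point is clear, with no radius limit.
; Each sampled point is printed and drawn as a debug circle.
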(event Custom|OnPerformSkill
  (bind _skillparameter (Variables|Default|GetSkillParameter))
  (bind (_starttransform _activator _targetlocation) (Utilities|Struct|BreakSkillParameter _skillparameter))
  (bind (_x _y) (Math|Vector|BreakVector _targetlocation))
  (bind _location (CallFunction|GetAvailableBlinkLocation (Math|Vector|MakeVector _x _y (.Z (Math|Vector|BreakVector (Transformation|GetActorLocation _activator)))) (Components|Capsule|GetScaledCapsuleRadius (Variables|/Script/Engine.Character|GetCapsuleComponent _activator))))
  (Transformation|SetActorLocation _activator _location false true)
  (CallFunction|WaitPostDelay))

(event EventBeginPlay
  (|CallParentFunction))

(event EventTick
  (params (DeltaSeconds :type Float%20%28single-precision%29))
  (|CallParentFunction 0.0))

(fn GetAvailableBlinkLocation
  (params (TargetLocation :type Vector) (ObjectRadius :type Float%20%28single-precision%29) (Character :type Character%20BP%20Object%20Reference))
  (bind _returnvalue (Class|KismetSystemLibrary|SphereOverlapActorsNEW TargetLocation ObjectRadius (LocalVariables|GetObjectTypeQuery) 0 (Utilities|Array|MakeArray Character)))
  (if _returnvalue
    (LocalVariables|SetRadius (+ (LocalVariables|GetRadius) (LocalVariables|GetRadiusIncrement)) :!label _label)
    (LocalVariables|SetDegree 0.0)
    (bind _output_get (LocalVariables|SetPoint (+ TargetLocation (* (Math|Vector|MakeVector (Math|Trig|Sin(Degrees) (LocalVariables|GetDegree)) (Math|Trig|Cos(Degrees) (LocalVariables|GetDegree)) 0.0) (LocalVariables|GetRadius))) :!label _label_2))
    (Development|PrintString (Utilities|String|ToString(Vector) (+ TargetLocation (* (Math|Vector|MakeVector (Math|Trig|Sin(Degrees) (LocalVariables|GetDegree)) (Math|Trig|Cos(Degrees) (LocalVariables|GetDegree)) 0.0) (LocalVariables|GetRadius)))) true true "(R=0.000000,G=0.660000,B=1.000000,A=1.000000)" 1e+02)
    (Rendering|Debug|DrawDebugCircle _output_get 1e+01 12 "(R=1.000000,G=1.000000,B=1.000000,A=1.000000)" 1e+02 0.0 "0.000000,1.000000,0.000000" "0.000000,0.000000,1.000000")
    (bind _returnvalue_2 (Class|KismetSystemLibrary|SphereOverlapActorsNEW _output_get ObjectRadius (LocalVariables|GetObjectTypeQuery) 0 (Utilities|Array|MakeArray Character)))
    (if _returnvalue_2
      (LocalVariables|SetDegree (+ (LocalVariables|GetDegree) (LocalVariables|GetDegreeIncrement)))
      (if (<= (LocalVariables|GetDegree) 3.6e+02)
        (goto _label_2)
        (else
          (goto _label)))
      (else
        (return (LocalVariables|GetPoint))))
    (else
      (return TargetLocation))))