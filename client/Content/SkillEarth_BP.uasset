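; Earth character skill that launches its activator in a frictionless charge along the start transform's forward vector, damaging an enemy it hits.
; On perform, it locks movement input, sets velocity, enables sphere overlaps, zeroes saved friction and braking, then binds actor hit and starts a timer.
; Any hit or timeout ends the charge, damaging only other-team characters.
; Ending restores movement, stops velocity and calls WaitPostDelay.
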(event Custom|OnPerformSkill
  (bind _skillparameter (Variables|Default|GetSkillParameter))
  (bind (_starttransform _activator) (Utilities|Struct|BreakSkillParameter _skillparameter))
  (Development|PrintText (Utilities|Text|ToText(String) _starttransform))
  (bind _ascharacter_earth_bp (Utilities|Casting|CastToCharacterEarth_BP _activator))
  (Variables|Default|SetActivator _ascharacter_earth_bp)
  (Utilities|FlowControl|Sequence
    (:then_0
      (Variables|/Game/Character_BP.Character_BP_C|SetIsMovable (Variables|Default|GetActivator) false))
    (:then_1
      (Variables|/Script/Engine.MovementComponent|SetVelocity (Variables|/Script/Engine.Character|GetCharacterMovement (Variables|Default|GetActivator)) (* (Math|Vector|GetForwardVector (.Rotation (Math|Transform|BreakTransform _starttransform))) (Variables|Default|GetVelocity))))
    (:then_2
      (Variables|/Script/Engine.PrimitiveComponent|SetbGenerateOverlapEvents (Variables|/Game/Character_BP.Character_BP_C|GetSphereMesh (Variables|Default|GetActivator)) true))
    (:then_3
      (Utilities|FlowControl|Sequence
        (:then_0
          (Variables|Default|SetPrevGroundFriction (Variables|/Script/Engine.CharacterMovementComponent|GetGroundFriction (Variables|/Script/Engine.Character|GetCharacterMovement (Variables|Default|GetActivator)))))
        (:then_1
          (Variables|Default|SetPrevBrakingDecelerationWalking (Variables|/Script/Engine.CharacterMovementComponent|GetBrakingDecelerationWalking (Variables|/Script/Engine.Character|GetCharacterMovement (Variables|Default|GetActivator)))))
        (:then_2
          (Variables|/Script/Engine.CharacterMovementComponent|SetGroundFriction (Variables|/Script/Engine.Character|GetCharacterMovement (Variables|Default|GetActivator)) 0.0))
        (:then_3
          (Variables|/Script/Engine.CharacterMovementComponent|SetBrakingDecelerationWalking (Variables|/Script/Engine.Character|GetCharacterMovement (Variables|Default|GetActivator)) 0.0))))
    (:then_4
      (Collision|AssignOnActorHit (Variables|Default|GetActivator) (delegate Custom|OnActorHit)))
    (:then_5
      (bind _returnvalue (Utilities|Time|SetTimerbyFunctionName self "OnEnd" (Variables|Default|GetActivatingTime)))
      (Variables|Default|SetTimer _returnvalue))))

(event Custom|OnEnd
  (bind _activator (Variables|Default|GetActivator))
  (bind _charactermovement (Variables|/Script/Engine.Character|GetCharacterMovement _activator))
  (Utilities|FlowControl|Sequence
    (:then_0
      (Collision|UnbindEventfromOnActorHit (Variables|Default|GetActivator) (delegate Custom|OnActorHit)))
    (:then_1
      (Utilities|Time|ClearandInvalidateTimerbyHandle (Variables|Default|GetTimer)))
    (:then_2
      (Variables|/Game/Character_BP.Character_BP_C|SetIsMovable (Variables|Default|GetActivator) true))
    (:then_3
      (Variables|/Script/Engine.MovementComponent|SetVelocity (Variables|/Script/Engine.Character|GetCharacterMovement (Variables|Default|GetActivator)) "0, 0, 0"))
    (:then_4
      (Variables|/Script/Engine.PrimitiveComponent|SetbGenerateOverlapEvents (Variables|/Game/Character_BP.Character_BP_C|GetSphereMesh (Variables|Default|GetActivator)) false))
    (:then_5
      (Variables|/Script/Engine.CharacterMovementComponent|SetGroundFriction _charactermovement (Variables|Default|GetPrevGroundFriction))
      (Variables|/Script/Engine.CharacterMovementComponent|SetBrakingDecelerationWalking _charactermovement (Variables|Default|GetPrevBrakingDecelerationWalking)))
    (:then_6
      (CallFunction|WaitPostDelay))))

(event Custom|OnActorHit
  (params (SelfActor :type Actor%20Object%20Reference) (OtherActor :type Actor%20Object%20Reference) (NormalImpulse :type Vector) (Hit :type Hit%20Result%20Structure%20%28by%20ref%29))
  (Development|PrintText "Earth Hit da Hit!" true true "(R=1.000000,G=0.790847,B=0.000000,A=1.000000)" 1e+01)
  (bind _ascharacter_bp (Utilities|Casting|CastToCharacter_BP OtherActor)
    (:then
      (Utilities|EqualBranch(Integer) (Variables|/Game/Character_BP.Character_BP_C|GetTeamID _ascharacter_bp) (Variables|/Game/Character_BP.Character_BP_C|GetTeamID (Variables|Default|GetActivator))
        (:True
          (CallFunction|OnEnd))
        (:False
          (CallFunction|DealDamage (Variables|Default|GetDamage) _ascharacter_bp)
          (CallFunction|OnEnd))))
    (:CastFailed
      (CallFunction|OnEnd))))

(event EventBeginPlay
  (|CallParentFunction))

(event EventTick
  (params (DeltaSeconds :type Float%20%28single-precision%29))
  (|CallParentFunction 0.0))