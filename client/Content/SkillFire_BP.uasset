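; Fire skill Blueprint that creates a line of timed explosions along the forward vector of a starting transform.
; ActivateSkillFire stores that transform before calling the parent activation, while plain ActivateSkill is overridden to print an error and fail.
; OnPerformSkill spawns all SkillFireExplosion_BP actors in one loop, with index-based spacing and staggered activation delays.
; It then waits for the last explosion's delay before calling WaitPostDelay.
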(event Custom|OnPerformSkill
  (bind _explosioncount (Variables|Default|GetExplosionCount))
  (Development|PrintText "SkillFire OnPerformSkill" true true "(R=0.000000,G=0.660000,B=1.000000,A=1.000000)" 1e+02)
  (for _index (range 1 _explosioncount)
    (bind _transform (CallFunction|CalculateExplosionTransformbyIndex _index))
    (bind _delay (CallFunction|CalculateExplosionDelaybyIndex _index))
    (Game|SpawnActorfromClass "/Game/SkillFireExplosion_BP.SkillFireExplosion_BP_C" _transform "Undefined" (Game|GetGameMode) _delay 0))
  (bind _delay_2 (CallFunction|CalculateExplosionDelaybyIndex _explosioncount))
  (Utilities|FlowControl|Delay _delay_2)
  (CallFunction|WaitPostDelay))

(event EventBeginPlay)

(event EventTick
  (params (DeltaSeconds :type Float%20%28single-precision%29))
  (|CallParentFunction DeltaSeconds))

(fn ActivateSkillFire
  (params (Transform :type Transform))
  (Variables|Default|SetStartingTransform Transform)
  (bind _isactivated (|CallParentFunction))
  (return _isactivated))

(fn ActivateSkill
  (Development|PrintText "ERROR : Use ActivateSkillFire Instead of ActivateSkill")
  (return false))

(fn CalculateExplosionDelaybyIndex
  (params (Index%28StartWith1%29 :type Integer))
  (return (+ (* (- Index%28StartWith1%29 1) (Variables|Default|GetExplosionDelay)) (Variables|Default|GetExplosionFirstDelay))))

(fn CalculateExplosionTransformbyIndex
  (params (Index%28StartWith1%29 :type Integer))
  (bind _startingtransform (Variables|Default|GetStartingTransform))
  (return (Math|Transform|MakeTransform (+ (.location _startingtransform) (* (Math|Vector|GetForwardVector (.rotation _startingtransform)) (* (- Index%28StartWith1%29 1) (Variables|Default|GetExplosionDistanceInterval)))) "0, 0, 0" "1,1,1")))