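; Wind skill Blueprint that fires a wind bullet when the skill is performed.
; On OnPerformSkill it spawns BulletSkillWind_BP at the skill parameter's start transform, owned by the game mode and tagged with the activator's team ID, then waits out the post delay.
; It also prints the start transform on screen as debug text; BeginPlay and Tick are disabled stubs.
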(event Custom|OnPerformSkill
  (bind _skillparameter (Variables|Default|GetSkillParameter))
  (bind (_starttransform _activator) (Utilities|Struct|BreakSkillParameter _skillparameter))
  (Development|PrintText (Utilities|Text|ToText(String) _starttransform) true true "(R=1.000000,G=0.000000,B=0.272645,A=1.000000)" 1e+02)
  (Game|SpawnActorfromClass "/Game/BulletSkillWind_BP.BulletSkillWind_BP_C" _starttransform "Undefined" (Game|GetGameMode) 0.0 (Variables|/Game/Character_BP.Character_BP_C|GetTeamID _activator))
  (CallFunction|WaitPostDelay))

(event EventBeginPlay
  (|CallParentFunction))

(event EventTick
  (params (DeltaSeconds :type Float%20%28single-precision%29))
  (|CallParentFunction 0.0))