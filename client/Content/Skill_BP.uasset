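; Skill_BP is a skill Blueprint, apparently a parent class, that gates activation and sequences pre- and post-delays around the skill's execution.
; ActivateSkill succeeds only when idle, then runs OnPerformSkill immediately or via a pre-delay timer.
; OnPerformSkill holds only a debug print before starting the post-delay, whose completion clears the activating flag.
; Tick counts down the remaining post-delay alongside that timer.
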(event Custom|OnPerformSkill
  (Development|PrintText "parent" true true "(R=0.000000,G=0.660000,B=1.000000,A=1.000000)" 1e+02)
  (CallFunction|WaitPostDelay))

(event EventBeginPlay)

(event EventTick
  (params (DeltaSeconds :type Float%20%28single-precision%29))
  (if (> (Variables|Default|GetRemainingPostDealyTime) 0.0)
    (Variables|Default|SetRemainingPostDealyTime (Math|Float|Max(Float) (- (Variables|Default|GetRemainingPostDealyTime) DeltaSeconds) 0.0))))

(fn ActivateSkill
  (Development|PrintText "Activate Skill" true true "(R=0.000000,G=0.660000,B=1.000000,A=1.000000)" 1e+02)
  (bind _isactivatable (CallFunction|IsActivatable))
  (if _isactivatable
    (Variables|Default|SetIsActivating true)
    (CallFunction|WaitPreDelay)
    (return true)
    (else
      (return false))))

(fn IsActivatable
  (return (and (<= (Variables|Default|GetRemainingPostDealyTime) 0.0) (not (Variables|Default|GetIsActivating)))))

(fn WaitPreDelay
  (bind _predelaytime (Variables|Default|GetPreDelayTime))
  (Development|PrintText "PreDelay" true true "(R=0.000000,G=0.660000,B=1.000000,A=1.000000)" 1e+02)
  (if (<= _predelaytime 0.0)
    (CallFunction|OnPerformSkill)
    (else
      (Utilities|Time|SetTimerbyFunctionName self "OnPerformSkill" _predelaytime))))

(fn WaitPostDelay
  (bind _postdelaytime (Variables|Default|GetPostDelayTime))
  (Development|PrintText "Wait Post Delay" true true "(R=0.000000,G=0.660000,B=1.000000,A=1.000000)" 1e+02)
  (Variables|Default|SetRemainingPostDealyTime _postdelaytime)
  (if (<= _postdelaytime 0.0)
    (CallFunction|OnPostDelayFinished)
    (else
      (Utilities|Time|SetTimerbyFunctionName self "OnPostDelayFinished" _postdelaytime))))

(fn OnPostDelayFinished
  (Development|PrintText "On Post Delay Finished" true true "(R=0.000000,G=0.660000,B=1.000000,A=1.000000)" 1e+02)
  (Variables|Default|SetRemainingPostDealyTime 0.0)
  (Variables|Default|SetIsActivating false))